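; Fadeable mesh object whose material opacity animates when StartFade or EndFade is called.
; The construction script applies the chosen mesh and creates a dynamic instance of the fade material on its first slot.
; EndFade plays a timeline forward and StartFade reverses it, with updates driving the "opac" parameter from the track scaled by a fade amount.
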(event EventEndFade
  (bind _newtrack_0 (Timeline|fadetime Play)
    (:Update
      (Rendering|Material|SetScalarParameterValue (Variables|Default|Getdynamicmat) "opac" (stale _result) :!class /Script/Engine.MaterialInstanceDynamic))))

(event EventStartFade
  (bind _newtrack_0 (Timeline|fadetime Reverse)
    (:Update
      (Rendering|Material|SetScalarParameterValue (Variables|Default|Getdynamicmat) "opac" (stale _result) :!class /Script/Engine.MaterialInstanceDynamic))))

(fn ConstructionScript
  (Components|StaticMesh|SetStaticMesh (Variables|Default|GetStaticMesh) (Variables|Default|GetmeshToUse))
  (bind _returnvalue (Rendering|Material|CreateDynamicMaterialInstance (Variables|Default|GetfadeMaterial) "None" "None" :!class /Script/Engine.KismetMaterialLibrary))
  (bind _output_get (Variables|Default|Setdynamicmat _returnvalue))
  (Rendering|Material|SetMaterial (Variables|Default|GetStaticMesh) 0 _output_get))