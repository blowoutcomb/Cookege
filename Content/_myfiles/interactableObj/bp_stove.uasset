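; Interactable stove that turns food items into ConeGuy actors, with placeholder HUD text for its Off and Cooking states.
; Interact toggles the state and plays or reverses a timeline that pitches the Stovetop.
; Each timeline finish flips a FlipFlop that shows or hides the Trigger and its collision, which starts disabled.
; When a fooditemTest overlaps the actor, it is destroyed after brief delays and a ConeGuy spawns at the Trigger.
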(event `/Game/_myfiles/bps/i_interactable.showInfo`
  (params (hud :type "/Game/_myfiles/widget/wbp_HUD Object Reference"))
  (switch `/Game/_myfiles/interactableObj/en_stoveStat` (`self.status`)
    (:`NewEnumerator0`
      (`/Game/_myfiles/widget/wbp_HUD.setinfotext` hud "aaaaaaaaaaaaaa"))
    (:`NewEnumerator1`
      (`/Game/_myfiles/widget/wbp_HUD.setinfotext` hud "eeeeeeeeeeeeeeeee"))))

(event `self.ReceiveBeginPlay`
  (`SceneComponent.SetVisibility` (`self.trigger`) false false)
  (`PrimitiveComponent.SetCollisionEnabled` (`self.trigger`) "NoCollision"))

(event `/Game/_myfiles/bps/i_interactable.interact`
  (switch `/Game/_myfiles/interactableObj/en_stoveStat` (`self.status`)
    (:`NewEnumerator0`
      (set `self.status` "NewEnumerator1")
      (bind (_direction _stoveon) (`Timeline|stovecooking` :!label _label)
        (:`Update`
          (`SceneComponent.K2_SetRelativeRotation` (`self.stovetop`) (`KismetMathLibrary.MakeRotator` 0.0 _stoveon) false false))
        (:`Finished`
          (`/Engine/EditorBlueprintResources/StandardMacros.FlipFlop`
            (:`A`
              (`SceneComponent.SetVisibility` (`self.trigger`) true false)
              (`PrimitiveComponent.SetCollisionEnabled` (`self.trigger`) "QueryAndPhysics"))
            (:`B`
              (`SceneComponent.SetVisibility` (`self.trigger`) false false)
              (`PrimitiveComponent.SetCollisionEnabled` (`self.trigger`) "NoCollision"))))))
    (:`NewEnumerator1`
      (set `self.status` "NewEnumerator0")
      (goto _label :!via `Reverse`))))

(event `self.ReceiveActorBeginOverlap`
  (params (OtherActor :type "Actor Object Reference"))
  (bind _asfooditem_test (cast `/Game/_myfiles/interactableObj/fooditemTest` OtherActor))
  (`KismetSystemLibrary.Delay` 0.2)
  (`self.K2_DestroyActor` _asfooditem_test)
  (`KismetSystemLibrary.Delay` 0.5)
  (`|SpawnActorFromClass` "/Game/_myfiles/bps/coneGuy.coneGuy_C" (`KismetMathLibrary.Conv_VectorToTransform` (`SceneComponent.K2_GetComponentLocation` (`self.trigger`))) "Undefined" "OverrideRootScale" null null))

(fn `UserConstructionScript`)